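; Bullet Bill item actor whose skeletal mesh flies along a spline path once play begins.
; BeginPlay calls Move, which plays a timeline whose track value is scaled by the length of a referenced Spline object's spline.
; Each update sets the mesh's world location and rotation from that distance along the spline, with scale fixed at one and no sweep.
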(event `Move`
  (bind _spline (`self.Spline`))
  (bind (_direction _movement_spline_track) (`Timeline|Timeline_0`)
    (:`Update`
      (bind _returnvalue (* _movement_spline_track (`SplineComponent.GetSplineLength` (`/Game/Kart/KartV4/Blueprints/KartV4AIPath.Spline` _spline))))
      (`SceneComponent.K2_SetWorldTransform` (`self.SkeletalMesh`) (`KismetMathLibrary.MakeTransform` (`SplineComponent.GetLocationAtDistanceAlongSpline` (`/Game/Kart/KartV4/Blueprints/KartV4AIPath.Spline` _spline) _returnvalue "World") (`SplineComponent.GetRotationAtDistanceAlongSpline` (`/Game/Kart/KartV4/Blueprints/KartV4AIPath.Spline` _spline) _returnvalue "World")) false false))))

(event `self.ReceiveBeginPlay`
  (`self.Move`))

(fn `UserConstructionScript`)