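; Water tanker hazard that periodically shows a puddle which damages player karts.
; WaterHazard starts on BeginPlay and calls itself after fixed delays, alternately hiding and showing the Water component and setting IsPuddleVisible to match.
; The Box begin-overlap event deals damage to a KartV4Player only while that flag is set, then prints debug health text.
; Damage triggers only on entry, so a kart already inside when the puddle appears is unharmed.
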(event `self.Box.OnComponentBeginOverlap`
  (params (OverlappedComponent :type "PrimitiveComponent Object Reference") (OtherActor :type "Actor Object Reference") (OtherComp :type "PrimitiveComponent Object Reference") (OtherBodyIndex :type Integer) (bFromSweep :type Boolean) (SweepResult :type "HitResult Structure (by ref)"))
  ;[1 1 1] Kart damaged when player hits - Matthew Brinton
  (bind _askart_v4player (cast `/Game/Kart/KartV4/Blueprints/KartV4Player` OtherActor))
  (if (`self.IsPuddleVisible?`)
    (`/Game/Kart/KartV4/Blueprints/KartV4.DealDamage` _askart_v4player 1)
    (`KismetSystemLibrary.PrintString` (`KismetStringLibrary.Conv_IntToString` (`/Game/Kart/KartV4/Blueprints/KartV4.CurrentHealth` _askart_v4player)))
    (`KismetSystemLibrary.PrintString` "DAMAGED PLAYER" true true (struct :`R` 0.390625 :`B` 0.057031 :`A` 1.0))))

(event `self.ReceiveBeginPlay`
  ;[1 1 1] Plays Water Hazard on BeginPlay
  (`self.Water Hazard`))

(event `Water Hazard`
  ;[1 1 1] Makes puddle visible & invisible - Matthew Brinton
  (set `self.IsPuddleVisible?` false)
  (`SceneComponent.SetHiddenInGame` (`self.Water`) true false)
  (`KismetSystemLibrary.Delay` 2.0)
  (set `self.IsPuddleVisible?` true)
  (`SceneComponent.SetHiddenInGame` (`self.Water`) false false)
  (`KismetSystemLibrary.Delay` 2.0)
  (`self.Water Hazard`))

(fn `UserConstructionScript`)