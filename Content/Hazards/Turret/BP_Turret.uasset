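; Automated turret hazard that attacks the nearest vehicle it can see within sensing range.
; Each tick it picks a target via sphere overlap and line-of-sight checks, then turns its top mesh toward it at constant speed with clamped pitch.
; When cooled down and tightly aligned by a dot-product test, it fires a projectile burst from the left barrel socket using a self-re-entering DoN and Delay loop.
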(event `self.ReceiveTick`
  (params (DeltaSeconds :type "Float (single-precision)"))
  (`self.FindTarget`)
  (`self.Target`
    (:`then`
      (`self.TurretRotation` DeltaSeconds)
      (`self.UpdateFire`))
    (:`else`)))

(event `Fire`
  (set `self.TimeOfLastFire` (`KismetSystemLibrary.GetGameTimeInSeconds`))
  (`|ExecutionSequence`
    (:`then_0`
      (goto _label :!via `Reset`))
    (:`then_1`
      (`/Engine/EditorBlueprintResources/StandardMacros.Do N` 5 :!label _label ; Defines how many times it will fire
        (:`Exit`
          (`|SpawnActorFromClass` "/Game/Hazards/Turret/Turret_Projectile.Turret_Projectile_C" (`SceneComponent.GetSocketTransform` (`self.TurretBarrelLeft`) "SocketFire" "RTS_World") "Undefined" "OverrideRootScale" null null)
          (`KismetSystemLibrary.Delay` 0.2) ; Delays the next shot
          (goto _label))))))

(fn `FindTarget`
  (locals (BestDistance :type "Float (double-precision)") (CurrentDistance :type "Float (double-precision)") (BestTarget :type "Actor Object Reference") (CurrentTarget :type "Actor Object Reference"))
  (set `local.BestDistance` (+ (`self.SensingRange`) 1.0))
  (bind _outactors (`KismetSystemLibrary.SphereOverlapActors` (`self.K2_GetActorLocation`) (`self.SensingRange`) (`|MakeArray` "ObjectTypeQuery5" :!type "EObjectTypeQuery Enum") "/Script/Engine.Actor"))
  (for _array_element _outactors
    (bind _output_get (set `local.CurrentTarget` _array_element))
    (bind _output_get_2 (set `local.CurrentDistance` (`self.GetDistanceTo` _output_get self)))
    (if (or (< _output_get_2 (`local.BestDistance`)) (not (`KismetSystemLibrary.IsValid` (`local.BestTarget`))))
      (`/Game/Hazards/Turret/MyFunctionLibrary.HasLineOfSight` (`SceneComponent.K2_GetComponentLocation` (`self.StaticMeshTop`)) (`self.K2_GetActorLocation` (`local.CurrentTarget`)) (`|MakeArray` self (`local.CurrentTarget`) :!type "Actor Object Reference"))
      (if true
        (set `local.BestTarget` (`local.CurrentTarget`))
        (set `local.BestDistance` (`local.CurrentDistance`)))))
  (set `self.Target` (`local.BestTarget`)))

(fn `TurretRotation`
  (params (DeltaSeconds :type "Float (double-precision)"))
  (locals (NewRotation :type "Rotator Structure" :default (struct)))
  (bind _output_get (set `local.NewRotation` (`KismetMathLibrary.RInterpTo_Constant` (`SceneComponent.K2_GetComponentRotation` (`self.StaticMeshTop`)) (`KismetMathLibrary.FindLookAtRotation` (`SceneComponent.K2_GetComponentLocation` (`self.StaticMeshTop`)) (`self.K2_GetActorLocation` (`self.Target`))) (`local.DeltaSeconds`) (`self.RotateSpeed`))))
  (`SceneComponent.K2_SetWorldRotation` (`self.StaticMeshTop`) (`KismetMathLibrary.MakeRotator` (.roll _output_get) (`KismetMathLibrary.ClampAngle` (.pitch _output_get) -45.0 75.0) (.yaw _output_get)) false false))

(fn `UpdateFire`
  (if (> (- (`KismetSystemLibrary.GetGameTimeInSeconds`) (`self.TimeOfLastFire`)) (`self.RateOfFire`))
    (if (> (`KismetMathLibrary.Dot_VectorVector` (`KismetMathLibrary.GetDirectionUnitVector` (`SceneComponent.K2_GetComponentLocation` (`self.StaticMeshTop`)) (`self.K2_GetActorLocation` (`self.Target`))) (`SceneComponent.GetForwardVector` (`self.StaticMeshTop`))) 0.999)
      (`self.Fire`))))

(fn `UserConstructionScript`)