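; Short-lived projectile hazard, named for a thrower, that damages the KartV4Player on contact.
; On BeginPlay it caches the player pawn and sets a life span so it expires on its own.
; Overlap on its sphere deals damage to the kart player, destroys the projectile and prints debug messages with the player's current health.
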(event `self.ReceiveBeginPlay`
  (bind _askart_v4player (cast `/Game/Kart/KartV4/Blueprints/KartV4Player` (`GameplayStatics.GetPlayerPawn` 0)))
  (set `self.Player REF` _askart_v4player)
  (`self.SetLifeSpan` 1.8))

(event `self.Sphere1.OnComponentBeginOverlap`
  (params (OverlappedComponent :type "PrimitiveComponent Object Reference") (OtherActor :type "Actor Object Reference") (OtherComp :type "PrimitiveComponent Object Reference") (OtherBodyIndex :type Integer) (bFromSweep :type Boolean) (SweepResult :type "HitResult Structure (by ref)"))
  (bind _askart_v4player (cast `/Game/Kart/KartV4/Blueprints/KartV4Player` OtherActor))
  (`/Game/Kart/KartV4/Blueprints/KartV4.DealDamage` _askart_v4player 1)
  (`self.K2_DestroyActor`)
  (`KismetSystemLibrary.PrintString` (`KismetStringLibrary.Conv_IntToString` (`/Game/Kart/KartV4/Blueprints/KartV4.CurrentHealth` _askart_v4player)))
  (`KismetSystemLibrary.PrintString` "DAMAGED PLAYER" true true (struct :`R` 0.390625 :`B` 0.057031 :`A` 1.0)))

(fn `UserConstructionScript`)