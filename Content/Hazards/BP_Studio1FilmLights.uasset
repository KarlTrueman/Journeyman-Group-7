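; BP_Studio1FilmLights is a hazard actor for Studio 1 film lights that homes in on the player pawn once its EnteredArea flag is true.
; Each Tick it uses VInterpTo Constant to move at a fixed, fast speed toward the player's location until almost on top of it.
; Movement teleports without sweeping, so nothing blocks it, and this graph only reads EnteredArea, never sets it.
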(event `self.ReceiveTick`
  (params (DeltaSeconds :type "Float (single-precision)"))
  (bind _returnvalue (`self.K2_GetActorLocation`))
  (bind _returnvalue_2 (`self.K2_GetActorLocation` (`GameplayStatics.GetPlayerPawn` 0)))
  (if (`self.EnteredArea?`)
    (if (> (`KismetMathLibrary.Vector_Distance` _returnvalue _returnvalue_2) 2.0)
      (`self.K2_SetActorLocation` (`KismetMathLibrary.VInterpTo_Constant` _returnvalue _returnvalue_2 (`GameplayStatics.GetWorldDeltaSeconds`) 4000.0) false true))))

(fn `UserConstructionScript`)