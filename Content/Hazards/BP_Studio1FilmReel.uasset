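; Film reel hazard that moves back and forth along a set path and deals damage to a kart player that overlaps its box.
; A timeline, with play rate set from the travel time, lerps the reel's relative location and rotation from its start transform toward an offset Destination.
; When the timeline finishes, a delay runs and a FlipFlop alternates between reversing and replaying the movement.
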(event `self.ReceiveBeginPlay`
  (bind (_returnvalue_location _returnvalue_rotation) (`KismetMathLibrary.BreakTransform` (`SceneComponent.GetRelativeTransform` (`self.Reel`))))
  ;[1 1 1] Store the start position & Rotation - Matthew Brinton
  (set `self.StartPosition` _returnvalue_location)
  (set `self.StartRotation` _returnvalue_rotation)
  ;[1 1 1] Playback of Timeline with Travel Speed - Matthew Brinton
  (`TimelineComponent.SetPlayRate` (`self.Movement Timeline`) (/ 1.0 (`self.TravelTimeInSeconds`)))
  (`self.Start Reel Movement`))

(event `Start Reel Movement`
  (bind (_destination_location _destination_rotation) (`KismetMathLibrary.BreakTransform` (`self.Destination`)))
  (bind _startposition (`self.StartPosition`))
  (bind _startrotation (`self.StartRotation`))
  (bind (_direction _reel_movement) (`Timeline|Movement Timeline` :!label _label)
    (:`Update`
      (set `self.Reel Movement` _reel_movement)
      ;[1 1 1] Determines Destination Location - Matthew Brinton
      (`SceneComponent.K2_SetRelativeLocationAndRotation` (`self.Reel`) (`KismetMathLibrary.VLerp` _startposition (+ _startposition _destination_location) (`self.Reel Movement`)) (`KismetMathLibrary.RLerp` _startrotation (`KismetMathLibrary.ComposeRotators` _startrotation _destination_rotation) (`self.Reel Movement`)) false false))
    (:`Finished`
      ;[1 1 1] Pause - Reverses or Starts Reel Movement - Matthew Brinton
      (`KismetSystemLibrary.Delay` (`self.DelayOnMovement`))
      (`/Engine/EditorBlueprintResources/StandardMacros.FlipFlop`
        (:`A`
          (`self.Reverse Reel Movement`))
        (:`B`
          (`self.Start Reel Movement`))))))

(event `self.Box.OnComponentBeginOverlap`
  (params (OverlappedComponent :type "PrimitiveComponent Object Reference") (OtherActor :type "Actor Object Reference") (OtherComp :type "PrimitiveComponent Object Reference") (OtherBodyIndex :type Integer) (bFromSweep :type Boolean) (SweepResult :type "HitResult Structure (by ref)"))
  (bind _askart_v4player (cast `/Game/Kart/KartV4/Blueprints/KartV4Player` OtherActor))
  (`/Game/Kart/KartV4/Blueprints/KartV4.DealDamage` _askart_v4player 1))

(event `Reverse Reel Movement`
  (goto _label :!via `Reverse`))

(fn `UserConstructionScript`)