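; BP_Studio4FallingLights is a hazard actor that drops a film light rig as soon as play begins.
; BeginPlay stores FilmLight1's relative start transform, scales MovementTimeline's play rate by TravelTimeInSeconds and calls LightsFallingSTART.
; The timeline's ReelMovement track lerps the rig's location and rotation toward the Destination offset from that start.
; When the timeline finishes, the three spotlights drop to zero intensity.
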(event `self.ReceiveBeginPlay`
  (bind (_returnvalue_location _returnvalue_rotation) (`KismetMathLibrary.BreakTransform` (`SceneComponent.GetRelativeTransform` (`self.Film Light 1`))))
  ;[1 1 1] Store the start position & Rotation - Matthew Brinton
  (set `self.StartPosition` _returnvalue_location)
  (set `self.StartRotation` _returnvalue_rotation)
  ;[1 1 1] Playback of Timeline with Travel Speed - Matthew Brinton
  (`TimelineComponent.SetPlayRate` (`self.Movement Timeline`) (/ 1.0 (`self.TravelTimeInSeconds`)))
  (`self.Lights Falling START`))

(event `Lights Falling START`
  (bind (_destination_location _destination_rotation) (`KismetMathLibrary.BreakTransform` (`self.Destination`)))
  (bind _startposition (`self.StartPosition`))
  (bind _startrotation (`self.StartRotation`))
  (bind (_direction _reel_movement) (`Timeline|Movement Timeline`)
    (:`Update`
      (set `self.Light Beam Movement` _reel_movement)
      ;[1 1 1] Determines Destination Location - Matthew Brinton
      (`SceneComponent.K2_SetRelativeLocationAndRotation` (`self.Film Light 1`) (`KismetMathLibrary.VLerp` _startposition (+ _startposition _destination_location) (`self.Light Beam Movement`)) (`KismetMathLibrary.RLerp` _startrotation (`KismetMathLibrary.ComposeRotators` _startrotation _destination_rotation) (`self.Light Beam Movement`)) false false))
    (:`Finished`
      (`LightComponent.SetIntensity` (`self.SpotLight`) 0.0)
      (`LightComponent.SetIntensity` (`self.SpotLight 2`) 0.0)
      (`LightComponent.SetIntensity` (`self.SpotLight 3`) 0.0))))

(fn `UserConstructionScript`)