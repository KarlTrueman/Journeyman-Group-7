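; BP_Studio1BoomMic is a boom mic hazard that chases the player's kart once its EnteredArea flag is true.
; BeginPlay caches the player pawn as a KartV4Player reference.
; While the flag is set, Tick moves the mic toward the pawn at constant speed with sweep collision and slowly interpolates its yaw to face the kart.
; Nothing in this graph sets EnteredArea.
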(event `self.ReceiveTick`
  (params (DeltaSeconds :type "Float (single-precision)"))
  (bind _returnvalue (`self.K2_GetActorLocation`))
  (bind _returnvalue_2 (`self.K2_GetActorLocation` (`GameplayStatics.GetPlayerPawn` 0)))
  (bind (_returnvalue_roll _returnvalue_pitch _returnvalue_yaw) (`KismetMathLibrary.BreakRotator` (`KismetMathLibrary.RInterpTo` (`self.K2_GetActorRotation`) (`KismetMathLibrary.FindLookAtRotation` (`self.K2_GetActorLocation`) (`self.K2_GetActorLocation` (`self.Character REF`))) (`GameplayStatics.GetWorldDeltaSeconds`) 0.5)))
  (if (`self.EnteredArea?`)
    (if (> (`KismetMathLibrary.Vector_Distance` _returnvalue _returnvalue_2) 1.0)
      (`self.K2_SetActorLocation` (`KismetMathLibrary.VInterpTo_Constant` _returnvalue _returnvalue_2 (`GameplayStatics.GetWorldDeltaSeconds`) 1000.0) true)
      (`self.K2_SetActorRotation` (`KismetMathLibrary.MakeRotator` 0.0 0.0 _returnvalue_yaw)))))

(event `self.ReceiveBeginPlay`
  (bind _askart_v4player (cast `/Game/Kart/KartV4/Blueprints/KartV4Player` (`GameplayStatics.GetPlayerPawn` 0)))
  (set `self.Character REF` _askart_v4player))

(fn `UserConstructionScript`)