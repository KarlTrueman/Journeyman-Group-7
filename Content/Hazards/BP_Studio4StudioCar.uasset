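; Studio car hazard Blueprint that moves a skeletal mesh car along a spline, starting on BeginPlay.
; The Movement timeline's track scales the spline length into a distance, which sets the mesh's world position and rotation each update at unit scale, without sweep.
; On Finished, the move event calls itself to repeat, using Play rather than PlayFromStart.
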(event `Move Studio Car Along Spine`
  (bind _spline (`self.Spline`))
  ;[1 1 1] Spline Movement - Matthew Brinton
  (bind (_direction _movement_spline_track) (`Timeline|Movement`)
    (:`Update`
      (bind _returnvalue (* _movement_spline_track (`SplineComponent.GetSplineLength` _spline)))
      (`SceneComponent.K2_SetWorldTransform` (`self.SkeletalMesh`) (`KismetMathLibrary.MakeTransform` (`SplineComponent.GetLocationAtDistanceAlongSpline` _spline _returnvalue "World") (`SplineComponent.GetRotationAtDistanceAlongSpline` _spline _returnvalue "World")) false false))
    (:`Finished`
      (`self.Move Studio Car Along Spine`))))

(event `self.ReceiveBeginPlay`
  ;[1 1 1] Starts Spline movement on BeginPlay - Matthew Brinton
  (`self.Move Studio Car Along Spine`))

(fn `UserConstructionScript`)