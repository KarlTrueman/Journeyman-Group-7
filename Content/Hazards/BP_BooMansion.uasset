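; BP_BooMansion is a moving Boo hazard that deals damage to a player kart overlapping its box.
; On BeginPlay, once the player pawn casts to KartV4Player, it caches the mesh's starting transform and scales timeline play rate by travel time.
; The timeline lerps the mesh, with sweep, toward a Destination offset from that start.
; When it finishes, a delay and FlipFlop alternate reverse and forward play, creating a ping-pong patrol.
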(event `self.ReceiveBeginPlay`
  (bind (_returnvalue_location _returnvalue_rotation) (`KismetMathLibrary.BreakTransform` (`SceneComponent.GetRelativeTransform` (`self.Boo Mesh`))))
  (bind _askart_v4player (cast `/Game/Kart/KartV4/Blueprints/KartV4Player` (`GameplayStatics.GetPlayerPawn` 0)))
  (set `self.Kart REF` _askart_v4player)
  ;[1 1 1] Store the start position & Rotation - Matthew Brinton
  (set `self.StartPosition` _returnvalue_location)
  (set `self.StartRotation` _returnvalue_rotation)
  ;[1 1 1] Playback of Timeline with Travel Speed - Matthew Brinton
  (`TimelineComponent.SetPlayRate` (`self.Boo Movement Timeline`) (/ 1.0 (`self.TravelTimeInSeconds`)))
  (`self.Start Movement - BOO`))

(event `self.Box.OnComponentBeginOverlap`
  (params (OverlappedComponent :type "PrimitiveComponent Object Reference") (OtherActor :type "Actor Object Reference") (OtherComp :type "PrimitiveComponent Object Reference") (OtherBodyIndex :type Integer) (bFromSweep :type Boolean) (SweepResult :type "HitResult Structure (by ref)"))
  (bind _askart_v4player (cast `/Game/Kart/KartV4/Blueprints/KartV4Player` OtherActor))
  (`/Game/Kart/KartV4/Blueprints/KartV4.DealDamage` _askart_v4player 1))

(event `Start Movement - BOO`
  (bind (_destination_location _destination_rotation) (`KismetMathLibrary.BreakTransform` (`self.Destination`)))
  (bind _startposition (`self.StartPosition`))
  (bind _startrotation (`self.StartRotation`))
  (bind (_direction _boo_movement) (`Timeline|Boo Movement Timeline` :!label _label)
    (:`Update`
      (set `self.Reverse Movement` _boo_movement)
      ;[1 1 1] Determines Destination Location - Matthew Brinton
      (`SceneComponent.K2_SetRelativeLocationAndRotation` (`self.Boo Mesh`) (`KismetMathLibrary.VLerp` _startposition (+ _startposition _destination_location) (`self.Reverse Movement`)) (`KismetMathLibrary.RLerp` _startrotation (`KismetMathLibrary.ComposeRotators` _startrotation _destination_rotation) (`self.Reverse Movement`)) true false))
    (:`Finished`
      ;[1 1 1] Pause - Reverses or Starts Reel Movement - Matthew Brinton
      (`KismetSystemLibrary.Delay` (`self.DelayOnMovement`))
      (`/Engine/EditorBlueprintResources/StandardMacros.FlipFlop`
        (:`A`
          (`self.Reverse Movement - BOO`))
        (:`B`
          (`self.Start Movement - BOO`))))))

(event `Reverse Movement - BOO`
  (goto _label :!via `Reverse`))

(fn `UserConstructionScript`)