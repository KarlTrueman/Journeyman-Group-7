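; BP_WaterTankerWater is a water puddle hazard that spreads after it spawns and damages the player kart on contact.
; A box overlap casts to KartV4Player, deals one damage and prints debug text with the kart's health.
; Tick drives PuddleIncrease, whose Delay throttles growth into fixed steps of X and Y scale until a size cap sets PuddleMaxSize.
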(event `self.Box.OnComponentBeginOverlap`
  (params (OverlappedComponent :type "PrimitiveComponent Object Reference") (OtherActor :type "Actor Object Reference") (OtherComp :type "PrimitiveComponent Object Reference") (OtherBodyIndex :type Integer) (bFromSweep :type Boolean) (SweepResult :type "HitResult Structure (by ref)"))
  ;[1 1 1] Damage Player Kart - Matthew Brinton
  (bind _askart_v4player (cast `/Game/Kart/KartV4/Blueprints/KartV4Player` OtherActor))
  (if true
    (`/Game/Kart/KartV4/Blueprints/KartV4.DealDamage` _askart_v4player 1)
    (`KismetSystemLibrary.PrintString` (`KismetStringLibrary.Conv_IntToString` (`/Game/Kart/KartV4/Blueprints/KartV4.CurrentHealth` _askart_v4player)))
    (`KismetSystemLibrary.PrintString` "DAMAGED PLAYER" true true (struct :`R` 0.390625 :`B` 0.057031 :`A` 1.0))))

(event `self.ReceiveTick`
  (params (DeltaSeconds :type "Float (single-precision)"))
  (`self.Puddle Increase`))

(event `Puddle Increase`
  (bind _returnvalue (`self.GetActorScale3D`))
  (`KismetSystemLibrary.Delay` 0.2)
  (bind _output_get (set `self.Puddle Size` (.x _returnvalue)))
  (if (>= _output_get 10.0)
    (set `self.PuddleMaxSize` true)
    (else
      (`self.SetActorScale3D` (+ _returnvalue (0.5 0.5 0.0))))))

(fn `UserConstructionScript`)