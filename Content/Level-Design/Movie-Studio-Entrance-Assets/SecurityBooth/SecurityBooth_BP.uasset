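; Security booth Blueprint for the movie studio entrance, with left and right gate arms that raise and lower.
; A timeline's Angle track, scaled by a separate open angle for each arm, sets each arm's world pitch, with roll and yaw zeroed.
; OpenGate plays the timeline and CloseGate reverses it.
; On BeginPlay the gate opens, then closes after a fixed delay, with no other trigger.
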(event `self.ReceiveBeginPlay`
  (`self.OpenGate`)
  (`KismetSystemLibrary.Delay` 5.0)
  (`self.CloseGate`))

(event `OpenGate`
  (bind (_direction _angle) (`Timeline|Timeline_0` :!label _label)
    (:`Update`
      (`SceneComponent.K2_SetWorldRotation` (`self.ArmLeft`) (`KismetMathLibrary.MakeRotator` 0.0 (* _angle (`self.OpenAngleLeft`))) false false)
      (`SceneComponent.K2_SetWorldRotation` (`self.ArmRight`) (`KismetMathLibrary.MakeRotator` 0.0 (* _angle (`self.OpenAngleRight`))) false false))))

(event `CloseGate`
  (goto _label :!via `Reverse`))

(fn `UserConstructionScript`)