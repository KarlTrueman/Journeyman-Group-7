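; StuntZoneBP is a trigger zone that refills kart boost while the player performs a stunt inside it.
; Begin and end overlap events set the InStuntZone flag on any Kart that enters or leaves.
; Tick reads player 0's kart and, when InStuntZone and Stunt are both true, adds BoostToAdd through AddingBoost, capped at MaxBoost.
; The gain is per frame, without delta-time scaling.
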(event `self.ReceiveActorBeginOverlap`
  (params (OtherActor :type "Actor Object Reference"))
  (bind _askart (cast `/Game/Kart/OldKartWrongScale/Kart` OtherActor))
  (set `/Game/Kart/OldKartWrongScale/Kart.In Stunt Zone` true _askart))

(event `self.ReceiveActorEndOverlap`
  (params (OtherActor :type "Actor Object Reference"))
  (bind _askart (cast `/Game/Kart/OldKartWrongScale/Kart` OtherActor))
  (set `/Game/Kart/OldKartWrongScale/Kart.In Stunt Zone` false _askart))

(event `self.ReceiveTick`
  (params (DeltaSeconds :type "Float (single-precision)"))
  (bind _askart (cast `/Game/Kart/OldKartWrongScale/Kart` (`GameplayStatics.GetPlayerPawn` 0)))
  (if (`/Game/Kart/OldKartWrongScale/Kart.In Stunt Zone` _askart)
    (if (`/Game/Kart/OldKartWrongScale/Kart.Stunt` _askart)
      (bind _boostoutput (`self.AddingBoost` (`/Game/Kart/OldKartWrongScale/Kart.Boost` _askart) (`/Game/Kart/OldKartWrongScale/Kart.MaxBoost` _askart)))
      (set `/Game/Kart/OldKartWrongScale/Kart.Boost` _boostoutput _askart))))

(fn `AddingBoost`
  (params (Boost :type Integer) (MaxBoost :type Integer))
  (returns (BoostOutput :type Integer))
  (bind _returnvalue (+ Boost (`self.Boost to add`)))
  ;[1 1 1] Function to add boost without going beyond max boost - Andrew
  (if (< _returnvalue MaxBoost)
    (return _returnvalue)
    (else
      (return MaxBoost))))

(fn `UserConstructionScript`)