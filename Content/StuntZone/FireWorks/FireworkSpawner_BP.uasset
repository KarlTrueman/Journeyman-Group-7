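; Fireworks spawner actor that keeps launching random firework Niagara effects around its location in the level.
; Tick feeds a short random Delay, which throttles spawning to irregular intervals.
; After each delay, it spawns a system picked at random from the Fireworks array, offset randomly on all three axes from the actor.
; The random index range runs up to the array length inclusive, so it can land out of bounds.
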(event `self.ReceiveTick`
  (params (DeltaSeconds :type "Float (single-precision)"))
  (bind (_returnvalue_x _returnvalue_y _returnvalue_z) (`KismetMathLibrary.BreakVector` (`self.K2_GetActorLocation`)))
  (bind _fireworks (`self.Fireworks`))
  ;[1 1 1] Fireworks (Kay Johnston)
  (`KismetSystemLibrary.Delay` (`KismetMathLibrary.RandomFloatInRange` 0.1 1.0))
  (`NiagaraFunctionLibrary.SpawnSystemAtLocation` (`|GetArrayItem` _fireworks (`KismetMathLibrary.RandomIntegerInRange` 0 (`KismetArrayLibrary.Array_Length` _fireworks))) (`KismetMathLibrary.MakeVector` (+ _returnvalue_x (`KismetMathLibrary.RandomFloatInRange` -500.0 500.0)) (+ (`KismetMathLibrary.RandomFloatInRange` -500.0 500.0) _returnvalue_y) (+ (`KismetMathLibrary.RandomFloatInRange` -500.0 500.0) _returnvalue_z))))

(fn `UserConstructionScript`)