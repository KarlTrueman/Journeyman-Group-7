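; Base kart Blueprint with arcade-style driving, mouse-controlled spring arm camera and basic health.
; Throttle and Steering ease speed and steering angle toward scaled inputs using FInterpTo.
; BaseClassTick, not called here, sweeps the kart along its arrow's forward vector and yaws it in proportion to speed and steering angle.
; DealDamage subtracts health and returns whether it is at or below MaxHealth, while AddHealth is empty.
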(event `InputAxisKey|MouseX`
  (params (AxisValue :type "Float (single-precision)"))
  (`SceneComponent.K2_AddRelativeRotation` (`self.SpringArm`) (`KismetMathLibrary.MakeRotator` 0.0 0.0 AxisValue) false false))

(event `InputAxisKey|MouseY`
  (params (AxisValue :type "Float (single-precision)"))
  (`SceneComponent.K2_AddRelativeRotation` (`self.SpringArm`) (`KismetMathLibrary.MakeRotator` 0.0 AxisValue) false false))

(fn `AddHealth`)

(fn `BaseClassTick`
  (bind (_returnvalue_roll _returnvalue_pitch _returnvalue_yaw) (`KismetMathLibrary.BreakRotator` (`self.K2_GetActorRotation`)))
  (bind _currentspeed (`self.CurrentSpeed`))
  (`self.K2_AddActorWorldOffset` (* (* (`SceneComponent.GetForwardVector` (`self.Arrow`)) _currentspeed) (`GameplayStatics.GetWorldDeltaSeconds`)) true)
  (`self.K2_SetActorRelativeRotation` (`KismetMathLibrary.MakeRotator` 0.0 0.0 (+ _returnvalue_yaw (* _currentspeed (`self.CurrentSteeringAngle`) (`self.SpeedToRotationFactor`) (`GameplayStatics.GetWorldDeltaSeconds`))))))

(fn `DealDamage`
  (params (Damage :type Integer))
  (returns (RespawnKart :type Boolean))
  (bind _output_get (set `self.CurrentHealth` (- (`self.CurrentHealth`) Damage)))
  (return (<= _output_get (`self.MaxHealth`))))

(fn `Steering`
  (params (SteeringAxis :type "Float (double-precision)"))
  (returns (CurrentSteeringAngle :type "Float (double-precision)"))
  (bind _output_get (set `self.CurrentSteeringAngle` (`KismetMathLibrary.FInterpTo` (`self.CurrentSteeringAngle`) (* SteeringAxis (`self.MaxSteeringAngle`)) (`GameplayStatics.GetWorldDeltaSeconds`) 4.0)))
  (return _output_get))

(fn `Throttle`
  (params (ThrottleInput :type "Float (double-precision)"))
  (returns (CurrentSpeed :type "Float (double-precision)"))
  (bind _output_get (set `self.CurrentSpeed` (`KismetMathLibrary.FInterpTo` (`self.CurrentSpeed`) (* ThrottleInput (`self.MaxSpeed`)) (`GameplayStatics.GetWorldDeltaSeconds`) 4.0)))
  (return _output_get))

(fn `UserConstructionScript`)