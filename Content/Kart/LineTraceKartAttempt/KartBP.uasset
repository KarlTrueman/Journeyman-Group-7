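; Kart Blueprint that drives by physics, with mouse-orbit camera and a rudimentary health system.
; Throttle and Steering ease speed and steering angle toward input-scaled limits; nothing here calls them or BaseClassTick.
; BaseClassTick pushes two spheres along the arrow's forward vector and yaws the actor by speed and steering.
; Offset movement and line-trace alignment are disconnected, AddHealth is empty, and DealDamage compares health to MaxHealth instead of zero.
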(event `InputAxisKey|MouseX`
  (params (AxisValue :type "Float (single-precision)"))
  (`SceneComponent.K2_AddRelativeRotation` (`self.SpringArm`) (`KismetMathLibrary.MakeRotator` 0.0 0.0 AxisValue) false false))

(event `InputAxisKey|MouseY`
  (params (AxisValue :type "Float (single-precision)"))
  (`SceneComponent.K2_AddRelativeRotation` (`self.SpringArm`) (`KismetMathLibrary.MakeRotator` 0.0 AxisValue) false false))

(fn `AddHealth`)

(fn `BaseClassTick`
  (bind (_returnvalue_roll _returnvalue_pitch _returnvalue_yaw) (`KismetMathLibrary.BreakRotator` (`self.K2_GetActorRotation`)))
  (bind _currentspeed (`self.CurrentSpeed`))
  (bind _returnvalue (* (* (* (`SceneComponent.GetForwardVector` (`self.Arrow`)) _currentspeed) (`GameplayStatics.GetWorldDeltaSeconds`)) 1000.0))
  (`PrimitiveComponent.AddForce` (`self.Sphere`) _returnvalue "None" false)
  (`PrimitiveComponent.AddForce` (`self.Sphere1`) _returnvalue "None" false)
  (`self.K2_SetActorRelativeRotation` (`KismetMathLibrary.MakeRotator` 0.0 0.0 (+ _returnvalue_yaw (* _currentspeed (`self.CurrentSteeringAngle`) (`self.SpeedToRotationFactor`) (`GameplayStatics.GetWorldDeltaSeconds`)))))
  (`self.BrokenLinetrace stuff`))

(fn `BrokenLinetrace stuff`)

(fn `DealDamage`
  (params (Damage :type Integer))
  (returns (RespawnKart :type Boolean))
  (bind _output_get (set `self.CurrentHealth` (- (`self.CurrentHealth`) Damage)))
  (return (<= _output_get (`self.MaxHealth`))))

(fn `Steering`
  (params (SteeringAxis :type "Float (double-precision)"))
  (returns (CurrentSteeringAngle :type "Float (double-precision)"))
  (bind _output_get (set `self.CurrentSteeringAngle` (`KismetMathLibrary.FInterpTo` (`self.CurrentSteeringAngle`) (* SteeringAxis (`self.MaxSteeringAngle`)) (`GameplayStatics.GetWorldDeltaSeconds`) 4.0)))
  (return _output_get))

(fn `Throttle`
  (params (ThrottleInput :type "Float (double-precision)"))
  (returns (CurrentSpeed :type "Float (double-precision)"))
  (bind _output_get (set `self.CurrentSpeed` (`KismetMathLibrary.FInterpTo` (`self.CurrentSpeed`) (* ThrottleInput (`self.MaxSpeed`)) (`GameplayStatics.GetWorldDeltaSeconds`) 4.0)))
  (return _output_get))

(fn `UserConstructionScript`)