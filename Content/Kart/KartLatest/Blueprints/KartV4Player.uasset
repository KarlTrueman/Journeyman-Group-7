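; Player kart Blueprint for an item-based racing game, feeding drive, drift, handbrake, boost and camera input into inherited kart logic.
; Timelines track race and lap times, with LapTimeCheck keeping the best lap.
; Use Item spawns bananas or shells, or fires the Clipper's sphere-overlap AOE, which calls Slowdown per vehicle found.
; Tick compares checkpoints for wrong-way warnings and shows a paused leaderboard when the lap counter hits four.
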(event `InputAction|Drift`
  (params (Key :type "Key Structure"))
  (bind _vehiclemovement (`self.VehicleMovement`))
  (bind _mesh (`self.Mesh`))
  (:`Pressed`
    (bind _returnvalue (`PrimitiveComponent.GetPhysicsLinearVelocity` _mesh "None"))
    (`self.Drift` true _returnvalue (`WheeledVehicleMovementComponent.GetCurrentGear` _vehiclemovement)))
  (:`Released`
    (bind _returnvalue_2 (`PrimitiveComponent.GetPhysicsLinearVelocity` _mesh "None"))
    (`self.Drift` false _returnvalue_2 (`WheeledVehicleMovementComponent.GetCurrentGear` _vehiclemovement))))

(event `InputAction|HandBrake`
  (params (Key :type "Key Structure"))
  (:`Pressed`
    (`self.Handbrake` true))
  (:`Released`
    (`self.Handbrake` false)))

(event `InputAxis|Throttle`
  (params (AxisValue :type "Float (single-precision)"))
  (if (`self.GamePlayingPlayer`)
    (if (not (`self.ThrottleOveride`))
      (`self.Throttle` AxisValue))))

(event `InputAxisKey|MouseX`
  (params (AxisValue :type "Float (single-precision)"))
  ;[0.8997 0.1041 1] Camera Stuff - Karl
  (`SceneComponent.K2_AddRelativeRotation` (`self.SpringArm`) (`KismetMathLibrary.MakeRotator` 0.0 0.0 AxisValue) false false))

(event `InputAction|Boost`
  (params (Key :type "Key Structure"))
  (:`Pressed`
    (if (`self.CanBoost`)
      (`self.Boost`))))

(event `InputAxis|Steering`
  (params (AxisValue :type "Float (single-precision)"))
  (bind _steeringoutput (`self.Steering` AxisValue))
  (if (or (> _steeringoutput 0.0) (< _steeringoutput 0.0))
    _))

(event `InputAxisKey|MouseY`
  (params (AxisValue :type "Float (single-precision)"))
  ;[0.8997 0.1041 1] Camera Stuff - Karl
  (`SceneComponent.K2_AddRelativeRotation` (`self.SpringArm`) (`KismetMathLibrary.MakeRotator` 0.0 AxisValue) false false))

(event `self.ReceiveTick`
  (params (DeltaSeconds :type "Float (single-precision)"))
  (`parent.ReceiveTick` DeltaSeconds)
  (if (== (`self.CurrentLapCounter`) 4)
    (bind _returnvalue (`|CreateWidget` "/Game/HUD/LeaderBoard.LeaderBoard_C"))
    (`GameplayStatics.SetGamePaused` true)
    (`UserWidget.AddToViewport` _returnvalue 0)
    (elif (> (`self.PreviousCheckPoint`) (`self.CurrentCheckPoint`))
      (bind _returnvalue_2 (`|CreateWidget` "/Game/HUD/RacePosition/WrongWay.WrongWay_C"))
      (`UserWidget.AddToViewport` _returnvalue_2 0)
      (set `self.WrongWay` true)
      (else
        (bind _foundwidgets (`WidgetBlueprintLibrary.GetAllWidgetsOfClass` "/Game/HUD/RacePosition/WrongWay.WrongWay_C"))
        (`Widget.RemoveFromParent` _foundwidgets)
        (set `self.WrongWay` false)))))

(event `StartRaceTime`
  ;[1 1 1] Handling of the total Race Time - Andrew
  (bind (_direction _time) (`Timeline|Timeline_2` :!label _label)
    (:`Update`
      (bind _output_get (set `self.RaceTime` _time))
      (set `self.RaceTimeText` (`self.TimeToText` _output_get)))))

(event `self.ReceiveBeginPlay`
  ;[1 1 1] MiniMap - Julia
  (bind _returnvalue (`|CreateWidget` "/Game/HUD/Minimap/Testing_minimap/Minimap_actual.Minimap_actual_C"))
  (`UserWidget.AddToViewport` _returnvalue 0))

(event `StopRaceTime`
  ;[1 1 1] Handling of the total Race Time - Andrew
  (goto _label :!via `Stop`))

(event `StartLapTime`
  ;[1 1 1] Handling of the Lap Time - Andrew
  (bind (_direction _time) (`Timeline|Timeline_3` :!via `PlayFromStart` :!label _label_2)
    (:`Update`
      (bind _output_get (set `self.CurrentLapTime` _time))
      (set `self.CurrentLapTimeText` (`self.TimeToText` _output_get)))))

(event `StopLapTime`
  ;[1 1 1] Handling of the Lap Time - Andrew
  (goto _label_2 :!via `Stop`))

(event `InputAction|Use Item`
  (params (Key :type "Key Structure"))
  (:`Pressed`
    (`|ExecutionSequence`
      (:`then_0`
        (switch `/Game/Items/Items` (`self.Item`)
          (:`NewEnumerator0`
            ;[1 1 1] Banana - Julia
            (if (`self.Has Bananana`)
              (`|SpawnActorFromClass` "/Game/Items/Bananana.Bananana_C" (`SceneComponent.K2_GetComponentToWorld` (`self.Banana spawn`)) "Undefined" "OverrideRootScale" null null)
              (set `self.Has Bananana` false)))
          (:`NewEnumerator1`
            ;[1 1 1] Shell - Julia
            (if (`self.Has Shell`)
              (`|SpawnActorFromClass` "/Game/Items/Red_Shell.Red_Shell_C" (`KismetMathLibrary.MakeTransform` (.location (`SceneComponent.K2_GetComponentToWorld` (`self.Shell spawn`))) (.rotation (`SceneComponent.K2_GetComponentToWorld` (`self.Shell spawn`))) (15.0 15.0 15.0)) "Undefined" "OverrideRootScale" null null)
              (set `self.Has Shell` false)))
          (:`NewEnumerator3`
            ;[1 1 1] Green Shell - Julia
            (if (`self.Has GreenShell`)
              (`|SpawnActorFromClass` "/Game/Items/Green_Shell.Green_Shell_C" (`KismetMathLibrary.MakeTransform` (.location (`SceneComponent.K2_GetComponentToWorld` (`self.Shell spawn`))) (.rotation (`SceneComponent.K2_GetComponentToWorld` (`self.Shell spawn`))) (15.0 15.0 15.0)) "Undefined" "OverrideRootScale" null null)
              (set `self.Has GreenShell` false)))
          (:`NewEnumerator4`
            ;[1 1 1] Clipper - Julia
            (if true
              (`self.Spawn AOE` (`self.K2_GetActorLocation`) 400.0 true self (delegate `CustomEvent_0`) 2.5 (struct :`G` 1.0 :`B` 0.091968 :`A` 1.0))))))
      (:`then_1`
        (set `self.Item` "NewEnumerator2")
        (set `self.ItemHeld` "")))))

(event `CustomEvent_0`
  (params (HitActor :type "Actor Object Reference"))
  ;[1 1 1] Clipper - Julia
)

(fn `LapTimeCheck`
  ;[1 1 1] LapTimeCheck - Andrew
  (`self.StopLapTime`)
  (if (== 0.0 (`self.BestLapTime`))
    (bind _output_get (set `self.BestLapTime` (`self.CurrentLapTime`) :!label _label))
    (set `self.BestLapText` (`self.TimeToText` _output_get))
    (set `self.CurrentLapTime` 0.0)
    (`self.StartLapTime`)
    (elif (> (`self.BestLapTime`) (`self.CurrentLapTime`))
      (goto _label)
      (else
        (set `self.CurrentLapTime` 0.0)
        (`self.StartLapTime`)))))

(fn `Spawn AOE`
  (params (Location :type "Vector Structure") (Radious :type "Float (double-precision)") (`Line of sight ` :type Boolean) (`AOE start ` :type "Actor Object Reference") (HitEvent :type "Delegate (by ref)") (`Debug duration` :type "Float (double-precision)") (`Debug colour` :type "LinearColor Structure"))
  (locals (`Current Actor ` :type "Actor Object Reference"))
  (add `self.AAOE hit` HitEvent)
  (`|ExecutionSequence`
    (:`then_0`
      (if (> (`local.Debug duration`) 0.0)
        (`KismetSystemLibrary.DrawDebugSphere` (`local.Location`) (`local.Radious`) 16 (`local.Debug colour`) (`local.Debug duration`) 2.0))
      (bind _outactors (`KismetSystemLibrary.SphereOverlapActors` (`local.Location`) (`local.Radious`) (`|MakeArray` "ObjectTypeQuery5" :!type "EObjectTypeQuery Enum") "/Script/Engine.Actor" (`|MakeArray` (`local.AOE start `))))
      (for _array_element _outactors
        (set `local.Current Actor ` _array_element)
        (`self.Slowdown` 0.0)
        (`self.AAOE hit` (`local.Current Actor `))))
    (:`then_1`
      (remove `self.AAOE hit` (`local.HitEvent`)))))

(fn `UserConstructionScript`
  (`parent.UserConstructionScript`))