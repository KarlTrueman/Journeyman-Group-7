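; Wheeled-vehicle kart pawn providing throttle, brake, steering, handbrake, boost, timed corner slowdown, and capped health and boost pools.
; Tick runs an all-wheels airborne check that gates interpolating roll and pitch toward level.
; Drift rebuilds the wheel setups with drifting classes on one side based on steering direction, then reapplies the supplied velocity and gear.
; Boost adds forward physics velocity, and two older anti-flip functions are marked unused.
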(event `InputAction|HandBrake`
  (params (Key :type "Key Structure"))
  (bind _vehiclemovement (`self.VehicleMovement`))
  ;[0.8997 0.1041 1] Controls - Karl
  (:`Pressed`
    (`WheeledVehicleMovementComponent.SetHandbrakeInput` _vehiclemovement true))
  (:`Released`
    (`WheeledVehicleMovementComponent.SetHandbrakeInput` _vehiclemovement false)))

(event `CornerSlow`
  (params (ThrottleInput :type "Float (double-precision)") (BrakeInput :type "Float (double-precision)") (ThrottleOutput :type "Float (double-precision)") (BrakeDuration :type "Float (double-precision)"))
  (`self.SlowdownMacro` ThrottleInput BrakeInput ThrottleOutput BrakeDuration))

(event `self.ReceiveTick`
  (params (DeltaSeconds :type "Float (single-precision)"))
  (bind (_returnvalue_roll _returnvalue_pitch _returnvalue_yaw) (`KismetMathLibrary.BreakRotator` (`self.K2_GetActorRotation`)))
  (bind _returnvalue (`GameplayStatics.GetWorldDeltaSeconds`))
  ;[0.8997 0.1041 1] Airtime - Karl
  (`self.AirTime`)
  (if (`self.InAir`)
    (`self.K2_SetActorRelativeRotation` (`KismetMathLibrary.MakeRotator` (`KismetMathLibrary.FInterpTo` _returnvalue_roll 0.0 _returnvalue (`self.Interp Speed`)) (`KismetMathLibrary.FInterpTo` _returnvalue_pitch 0.0 _returnvalue (`self.Interp Speed`)) _returnvalue_yaw) true true)))

(fn `AddBoost`
  (params (BoostValue :type Integer))
  (bind _returnvalue (+ BoostValue (`self.CurrentBoost`)))
  ;[0.8997 0.1041 1] AddBoost - Karl
  (if (>= _returnvalue (`self.MaxBoost`))
    (set `self.CurrentBoost` (`self.MaxBoost`))
    (else
      (set `self.CurrentBoost` _returnvalue))))

(fn `AddHealth`
  (params (HealthValue :type Integer))
  (bind _returnvalue (+ HealthValue (`self.CurrentHealth`)))
  ;[0.8997 0.1041 1] AddHealth - Karl
  (if (>= _returnvalue (`self.MaxHealth`))
    (set `self.CurrentHealth` (`self.MaxHealth`))
    (else
      (set `self.CurrentHealth` _returnvalue))))

(fn `AirTime`
  (locals (SetIsInAir :type Boolean :default true))
  ;[0.8997 0.1041 1] Air Time - Karl
  (for _array_element (`WheeledVehicleMovementComponent.Wheels` (`self.VehicleMovement`))
    (if (not (`VehicleWheel.IsInAir` _array_element))
      (set `local.SetIsInAir` false)))
  (if (`local.SetIsInAir`)
    (set `self.InAir` true)
    (else
      (set `self.InAir` false))))

(fn `AntiFlipV1(Unused)`
  (bind (_returnvalue_roll _returnvalue_pitch _returnvalue_yaw) (`KismetMathLibrary.BreakRotator` (`self.K2_GetActorRotation`)))
  ;[0.8997 0.1041 1] Antip Flip V1 - Karl
  (if (> _returnvalue_roll 20.0)
    (`self.K2_SetActorRelativeRotation` (`KismetMathLibrary.MakeRotator` (`KismetMathLibrary.FInterpTo` _returnvalue_roll 0.0 (`GameplayStatics.GetWorldDeltaSeconds`) 100.0) _returnvalue_pitch _returnvalue_yaw))))

(fn `AntiFlipV2(Unused)`
  (bind _roll (.roll (`self.K2_GetActorRotation`)))
  ;[0.8997 0.1041 1] AntipFlipV2 - Karl
  (if (> _roll 10.0)
    (set `self.RollRotation` 20.0)
    (`self.K2_SetActorRotation` (`KismetMathLibrary.MakeRotator` (`self.RollRotation`) (.pitch (`self.K2_GetActorRotation`)) (.yaw (`self.K2_GetActorRotation`))) true :!label _label)
    (`KismetSystemLibrary.PrintString` (`KismetStringLibrary.Conv_RotatorToString` (`self.K2_GetActorRotation`)))
    (elif (< _roll -10.0)
      (set `self.RollRotation` -20.0)
      (else
        (set `self.RollRotation` _roll)
        (goto _label)))))

(fn `Boost`
  (bind _returnvalue (* (`self.GetActorForwardVector`) 150.0))
  ;[0.8997 0.1041 1] Boost - Katl
  (if (< (`KismetMathLibrary.VSize` _returnvalue) (`self.MaxVelocity`))
    (`PrimitiveComponent.SetPhysicsLinearVelocity` (`MovementComponent.UpdatedPrimitive` (`self.VehicleMovement`)) _returnvalue true "None")))

(fn `Brake`
  (params (BrakeInput :type "Float (double-precision)"))
  (`WheeledVehicleMovementComponent.SetBrakeInput` (`self.VehicleMovement`) BrakeInput))

(fn `DealDamage`
  (params (Damage :type Integer))
  (returns (RespawnKart :type Boolean))
  ;[0.8997 0.1041 1] Deal Damage - Karl
  (bind _output_get (set `self.CurrentHealth` (- (`self.CurrentHealth`) Damage)))
  (return (<= _output_get 0)))

(fn `Drift`
  (params (IsDrifting :type Boolean) (Velocity :type "Vector Structure") (Gear :type Integer))
  (locals (FL :type Boolean) (FR :type Boolean) (RL :type Boolean) (RR :type Boolean))
  (bind _returnvalue (`self.GetInputAxisValue`))
  (if IsDrifting
    ;[1 1 1] If Steer Right
    (if (> _returnvalue 0.0)
      (set `local.FL` true)
      (set `local.FR` false)
      (set `local.RL` true)
      (set `local.RR` false)
      (`KismetSystemLibrary.PrintString` "Right")
      (`TireLib.modifyTyreConfig` (`self.VehicleMovement`) (`|MakeArray` (make `WheelSetupBp` (select `bool` (`local.FL`) :`false` "/Game/Kart/KartLatest/Blueprints/KartV4Wheels.KartV4Wheels_C" :`true` "/Game/Kart/KartLatest/Blueprints/KartV4WheelsDrifting.KartV4WheelsDrifting_C" :!type "VehicleWheel Class Reference") "FL") (make `WheelSetupBp` (select `bool` (`local.FR`) :`false` "/Game/Kart/KartLatest/Blueprints/KartV4Wheels.KartV4Wheels_C" :`true` "/Game/Kart/KartLatest/Blueprints/KartV4WheelsDrifting.KartV4WheelsDrifting_C" :!type "VehicleWheel Class Reference") "FR") (make `WheelSetupBp` (select `bool` (`local.RL`) :`false` "/Game/Kart/KartLatest/Blueprints/KartV4Wheels.KartV4Wheels_C" :`true` "/Game/Kart/KartLatest/Blueprints/KartV4WheelsDrifting.KartV4WheelsDrifting_C" :!type "VehicleWheel Class Reference") "RL" (0.0 0.0 0.0) true) (make `WheelSetupBp` (select `bool` (`local.RR`) :`false` "/Game/Kart/KartLatest/Blueprints/KartV4Wheels.KartV4Wheels_C" :`true` "/Game/Kart/KartLatest/Blueprints/KartV4WheelsDrifting.KartV4WheelsDrifting_C" :!type "VehicleWheel Class Reference") "RR" (0.0 0.0 0.0) true)) :!label _label)
      (`PrimitiveComponent.SetAllPhysicsLinearVelocity` (`self.Mesh`) Velocity false)
      (`WheeledVehicleMovementComponent.SetTargetGear` (`self.VehicleMovement`) Gear true)
      (else
        ;[1 1 1] If Steer Left
        (if (< _returnvalue 0.0)
          (set `local.FL` false)
          (set `local.FR` true)
          (set `local.RL` false)
          (set `local.RR` true)
          (`KismetSystemLibrary.PrintString` "Left")
          (goto _label)
          (elif (== _returnvalue 0.0)
            (set `local.FL` false)
            (set `local.FR` false)
            (set `local.RL` false)
            (set `local.RR` false)
            (`KismetSystemLibrary.PrintString` "Straight")
            (goto _label)))))
    (else
      (set `local.FL` false)
      (set `local.FR` false)
      (set `local.RL` false)
      (set `local.RR` false)
      (goto _label))))

(fn `Handbrake`
  (params (HandbrakeIn :type Boolean))
  ;[0.8997 0.1041 1] Handbrake - Karl
  (if HandbrakeIn
    (`WheeledVehicleMovementComponent.SetHandbrakeInput` (`self.VehicleMovement`) true)
    (else
      (`WheeledVehicleMovementComponent.SetHandbrakeInput` (`self.VehicleMovement`) false)))
  (return))

(fn `Slowdown`
  (params (ThrottleInput :type "Float (double-precision)") (ThrottleOutput :type "Float (double-precision)") (BrakeForce :type "Float (double-precision)") (BrakeLength :type "Float (double-precision)"))
  ;[0.8997 0.1041 1] Slowdown - Karl
  (`self.CornerSlow` ThrottleInput BrakeForce ThrottleOutput BrakeLength)
  (return))

(fn `Steering`
  (params (SteeringInput :type "Float (double-precision)"))
  (returns (SteeringOutput :type "Float (double-precision)"))
  ;[0.8997 0.1041 1] Steering - Karl
  (`WheeledVehicleMovementComponent.SetSteeringInput` (`self.VehicleMovement`) SteeringInput)
  (return SteeringInput))

(fn `Throttle`
  (params (ThrottleInput :type "Float (double-precision)"))
  (returns (ThrottleOutput :type "Float (double-precision)"))
  ;[0.8997 0.1041 1] Throttle - Karl
  (`WheeledVehicleMovementComponent.SetThrottleInput` (`self.VehicleMovement`) ThrottleInput)
  (return ThrottleInput))

(fn `UserConstructionScript`)