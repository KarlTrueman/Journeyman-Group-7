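; BoostToggle is a trigger Blueprint that enables or disables boosting for karts that enter it.
; When an actor overlaps its Box component, it casts to KartV4 and copies its own Boost flag into that kart's CanBoost.
; It then prints the kart's name with the resulting enabled or disabled state.
; The flag is only set on entry, with no end-overlap handling to revert it.
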(event `self.Box.OnComponentBeginOverlap`
  (params (OverlappedComponent :type "PrimitiveComponent Object Reference") (OtherActor :type "Actor Object Reference") (OtherComp :type "PrimitiveComponent Object Reference") (OtherBodyIndex :type Integer) (bFromSweep :type Boolean) (SweepResult :type "HitResult Structure (by ref)"))
  ;[0.8997 0.1041 1] Boost Toggle - Karl
  (bind _askart_v4 (cast `/Game/Kart/KartV4/Blueprints/KartV4` OtherActor))
  (bind _output_get (set `/Game/Kart/KartV4/Blueprints/KartV4.CanBoost` (`self.Boost`) _askart_v4))
  (if _output_get
    (`KismetSystemLibrary.PrintString` (`KismetStringLibrary.Concat_StrStr` (`KismetTextLibrary.Conv_TextToString` (`/Game/Kart/KartV4/Blueprints/KartV4.Name` _askart_v4)) ": " "Boost Enabled"))
    (else
      (`KismetSystemLibrary.PrintString` (`KismetStringLibrary.Concat_StrStr` (`KismetTextLibrary.Conv_TextToString` (`/Game/Kart/KartV4/Blueprints/KartV4.Name` _askart_v4)) ": " "Boost Disabled")))))

(fn `UserConstructionScript`)