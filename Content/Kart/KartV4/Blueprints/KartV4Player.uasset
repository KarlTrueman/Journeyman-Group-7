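; Player kart Blueprint that forwards driving, boost and handbrake input, and adds race HUD and item use.
; Timelines serve as race and lap stopwatches, with LapTimeCheck saving the best lap and restarting the lap timer.
; Tick compares checkpoints to toggle a wrong-way widget, and pauses the game with a leaderboard when the lap counter hits four.
; Use Item spawns the held red shell, banana or green shell at its spawn component.
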(event `InputAction|HandBrake`
  (params (Key :type "Key Structure"))
  (:`Pressed`
    (`self.Handbrake` true))
  (:`Released`
    (`self.Handbrake` false)))

(event `InputAxisKey|MouseX`
  (params (AxisValue :type "Float (single-precision)"))
  ;[1 1 1] Camera Stuff - Karl
)

(event `InputAction|Boost`
  (params (Key :type "Key Structure"))
  (:`Pressed`
    (`self.Boost`)))

(event `InputAxis|Throttle`
  (params (AxisValue :type "Float (single-precision)"))
  (if (not (`self.ThrottleOveride`))
    (`self.Throttle` AxisValue)))

(event `InputAxisKey|MouseY`
  (params (AxisValue :type "Float (single-precision)"))
  ;[1 1 1] Camera Stuff - Karl
)

(event `InputAxis|Steering`
  (params (AxisValue :type "Float (single-precision)"))
  (`self.Steering` AxisValue))

(event `self.ReceiveTick`
  (params (DeltaSeconds :type "Float (single-precision)"))
  (`parent.ReceiveTick` DeltaSeconds)
  (if (== (`self.CurrentLapCounter`) 4)
    (bind _returnvalue (`|CreateWidget` "/Game/HUD/LeaderBoard.LeaderBoard_C"))
    (`GameplayStatics.SetGamePaused` true)
    (`UserWidget.AddToViewport` _returnvalue 0)
    (elif (> (`self.PreviousCheckPoint`) (`self.CurrentCheckPoint`))
      (bind _returnvalue_2 (`|CreateWidget` "/Game/HUD/RacePosition/WrongWay.WrongWay_C"))
      (`UserWidget.AddToViewport` _returnvalue_2 0)
      (set `self.WrongWay` true)
      (else
        (bind _foundwidgets (`WidgetBlueprintLibrary.GetAllWidgetsOfClass` "/Game/HUD/RacePosition/WrongWay.WrongWay_C"))
        (`Widget.RemoveFromParent` _foundwidgets)
        (set `self.WrongWay` false)))))

(event `StartRaceTime`
  ;[1 1 1] Handling of the total Race Time - Andrew
  (bind (_direction _time) (`Timeline|Timeline_2` :!label _label)
    (:`Update`
      (bind _output_get (set `self.RaceTime` _time))
      (set `self.RaceTimeText` (`self.TimeToText` _output_get)))))

(event `self.ReceiveBeginPlay`
  ;[1 1 1] MiniMap - Julia
  (bind _returnvalue (`|CreateWidget` "/Game/HUD/Minimap/Testing_minimap/Minimap_actual.Minimap_actual_C"))
  (`UserWidget.AddToViewport` _returnvalue 0))

(event `StopRaceTime`
  ;[1 1 1] Handling of the total Race Time - Andrew
  (goto _label :!via `Stop`))

(event `StartLapTime`
  ;[1 1 1] Handling of the Lap Time - Andrew
  (bind (_direction _time) (`Timeline|Timeline_3` :!via `PlayFromStart` :!label _label_2)
    (:`Update`
      (bind _output_get (set `self.CurrentLapTime` _time))
      (set `self.CurrentLapTimeText` (`self.TimeToText` _output_get)))))

(event `StopLapTime`
  ;[1 1 1] Handling of the Lap Time - Andrew
  (goto _label_2 :!via `Stop`))

(event `InputAction|Use Item`
  (params (Key :type "Key Structure"))
  (:`Pressed`
    (switch `int` (`self.Item Index`)
      (:`0`
        ;[1 1 1] Shell - Julia
        (if (`self.Has Shell`)
          (`|SpawnActorFromClass` "/Game/Items/Red_Shell.Red_Shell_C" (`KismetMathLibrary.MakeTransform` (.location (`SceneComponent.K2_GetComponentToWorld` (`self.Shell spawn`))) (.rotation (`SceneComponent.K2_GetComponentToWorld` (`self.Shell spawn`))) (15.0 15.0 15.0)) "Undefined" "OverrideRootScale" null null)
          (set `self.Has Shell` false)
          (set `self.ItemHeld` "" :!label _label_3)))
      (:`1`
        ;[1 1 1] Banana - Julia
        (if (`self.Has Bananana`)
          (`|SpawnActorFromClass` "/Game/Items/Bananana.Bananana_C" (`SceneComponent.K2_GetComponentToWorld` (`self.Banana spawn`)) "Undefined" "OverrideRootScale" null null)
          (set `self.Has Bananana` false)
          (goto _label_3)))
      (:`2`
        ;[1 1 1] Green Shell - Julia
        (if (`self.Has GreenShell`)
          (`|SpawnActorFromClass` "/Game/Items/Green_Shell.Green_Shell_C" (`KismetMathLibrary.MakeTransform` (.location (`SceneComponent.K2_GetComponentToWorld` (`self.Shell spawn`))) (.rotation (`SceneComponent.K2_GetComponentToWorld` (`self.Shell spawn`))) (15.0 15.0 15.0)) "Undefined" "OverrideRootScale" null null)
          (set `self.Has GreenShell` false)
          (goto _label_3))))))

(fn `LapTimeCheck`
  ;[1 1 1] LapTimeCheck - Andrew
  (`self.StopLapTime`)
  (if (== 0.0 (`self.BestLapTime`))
    (bind _output_get (set `self.BestLapTime` (`self.CurrentLapTime`) :!label _label))
    (set `self.BestLapText` (`self.TimeToText` _output_get))
    (set `self.CurrentLapTime` 0.0)
    (`self.StartLapTime`)
    (elif (> (`self.BestLapTime`) (`self.CurrentLapTime`))
      (goto _label)
      (else
        (set `self.CurrentLapTime` 0.0)
        (`self.StartLapTime`)))))

(fn `UserConstructionScript`
  (`parent.UserConstructionScript`))