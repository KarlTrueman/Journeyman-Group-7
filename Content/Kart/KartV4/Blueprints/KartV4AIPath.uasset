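; Track path actor for kart races that supplies a spline to the race position UI.
; The construction script rebuilds SplineNew by resampling the Spline component at fixed distance intervals in world space, producing evenly spaced points.
; On BeginPlay it gathers all KartV4AI actors, creates a RacePosition widget with SplineNew, the player pawn and those AI karts, then adds it to the viewport.
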(event `self.ReceiveBeginPlay`
  (bind _outactors (`GameplayStatics.GetAllActorsOfClass` "/Game/Kart/KartV4/Blueprints/KartV4AI.KartV4AI_C"))
  (bind _returnvalue (`|CreateWidget` "/Game/HUD/RacePosition.RacePosition_C" null (`self.SplineNew`) (`GameplayStatics.GetPlayerPawn` 0)))
  (set `/Game/HUD/RacePosition.AiKarts` _outactors _returnvalue)
  (`UserWidget.AddToViewport` _returnvalue 0))

(fn `UserConstructionScript`
  (`SplineComponent.ClearSplinePoints` (`self.SplineNew`) true)
  (for _index (range (+ (`KismetMathLibrary.FTrunc` (/ (`SplineComponent.GetSplineLength` (`self.Spline`)) 100.0)) 1))
    (`SplineComponent.AddSplinePointAtIndex` (`self.SplineNew`) (`SplineComponent.GetLocationAtDistanceAlongSpline` (`self.Spline`) (* _index 100.0) "World") 0 "World" true)))