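; AI controller that drives a KartV4AI kart along a KartV4AIPath spline.
; On BeginPlay it applies full throttle to the controlled pawn.
; Each tick it takes the first path actor in the level, projects 500 units along the nearest spline tangent from the kart and snaps that point to the spline.
; The yaw difference toward this look-ahead target maps to a clamped, inverted steering input.
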(event `self.ReceiveTick`
  (params (DeltaSeconds :type "Float (single-precision)"))
  (bind _outactors (`GameplayStatics.GetAllActorsOfClass` "/Game/Kart/KartV4/Blueprints/KartV4AIPath.KartV4AIPath_C"))
  (bind _steeringoutput (`self.GetPath` _outactors))
  (`/Game/Kart/KartV4/Blueprints/KartV4.Steering` (stale `self.ReceiveBeginPlay` _askart_v4ai) _steeringoutput))

(event `self.ReceiveBeginPlay`
  (bind _askart_v4ai (cast `/Game/Kart/KartV4/Blueprints/KartV4AI` (`self.K2_GetPawn`)))
  (`/Game/Kart/KartV4/Blueprints/KartV4.Throttle` _askart_v4ai 1.0))

(fn `GetPath`
  (params (Splines :type "Array of /Game/Kart/KartV4/Blueprints/KartV4AIPath Object Reference"))
  (returns (SteeringOutput :type "Float (double-precision)"))
  (bind _returnvalue (`self.K2_GetPawn`))
  (bind _returnvalue_2 (`self.K2_GetActorLocation` _returnvalue))
  (bind _spline (`/Game/Kart/KartV4/Blueprints/KartV4AIPath.Spline` (`|GetArrayItem` Splines)))
  (bind (_returnvalue_roll _returnvalue_pitch _returnvalue_yaw) (`KismetMathLibrary.BreakRotator` (`KismetMathLibrary.NormalizedDeltaRotator` (`KismetMathLibrary.FindLookAtRotation` _returnvalue_2 (`SplineComponent.FindLocationClosestToWorldLocation` _spline (+ (* (`KismetMathLibrary.Normal` (`SplineComponent.FindTangentClosestToWorldLocation` _spline _returnvalue_2 "World")) 500.0) _returnvalue_2) "World")) (`self.K2_GetActorRotation` _returnvalue))))
  (return (`KismetMathLibrary.MapRangeClamped` _returnvalue_yaw -90.0 90.0 1.0 -1.0)))

(fn `UserConstructionScript`)