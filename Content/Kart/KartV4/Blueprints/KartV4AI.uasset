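; AI-driven kart that follows a track spline and can use random items.
; Each tick it projects a point ahead along the spline tangent, snaps it back to the spline, and maps the yaw difference toward it into steering input.
; AIstartgame applies full throttle.
; UseAnItem randomly grants and immediately uses a banana, green shell or red shell, printing the roll.
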(event `Use An Item`
  (bind _output_get (set `self.AI item selector` (`KismetMathLibrary.RandomIntegerInRange` 0 2)))
  (`KismetSystemLibrary.PrintString` (`KismetStringLibrary.Conv_IntToString` _output_get))
  (switch `int` _output_get
    (:`0`
      (set `self.Has Bananana` true)
      (`self.UseBanana`))
    (:`1`
      (set `self.Has GreenShell` true)
      (`self.UseGreenShell`))
    (:`2`
      (set `self.Has Shell` true)
      (`self.UseRedShell`))))

(event `self.ReceiveTick`
  (params (DeltaSeconds :type "Float (single-precision)"))
  (`parent.ReceiveTick` 0.0)
  (bind _steeringoutput (`self.GetPath` (`self.Splines`)))
  (`self.Steering` _steeringoutput))

(event `AI start game`
  (`self.Throttle` 1.0))

(fn `GetPath`
  (params (Splines :type "/Game/Kart/KartV4/Blueprints/KartV4AIPath Object Reference"))
  (returns (SteeringOutput :type "Float (double-precision)"))
  (bind _returnvalue (`self.K2_GetActorLocation`))
  (bind _spline (`/Game/Kart/KartV4/Blueprints/KartV4AIPath.Spline` Splines))
  (bind (_returnvalue_roll _returnvalue_pitch _returnvalue_yaw) (`KismetMathLibrary.BreakRotator` (`KismetMathLibrary.NormalizedDeltaRotator` (`KismetMathLibrary.FindLookAtRotation` _returnvalue (`SplineComponent.FindLocationClosestToWorldLocation` _spline (+ (* (`KismetMathLibrary.Normal` (`SplineComponent.FindTangentClosestToWorldLocation` _spline _returnvalue "World")) 500.0) _returnvalue) "World")) (`self.K2_GetActorRotation`))))
  ;[1 1 1] Get Path - Karl
  (return (`KismetMathLibrary.MapRangeClamped` _returnvalue_yaw 90.0 -90.0 1.0 -1.0)))

(fn `UserConstructionScript`
  (`parent.UserConstructionScript`))