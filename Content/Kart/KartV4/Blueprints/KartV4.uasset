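; KartV4 is the wheeled-vehicle kart for a Mario Kart-style racer, with items, health, boost and drifting.
; For players, the construction script reads Game Instance selections to apply data-table kart meshes and wheels, plus a seated character.
; Tick levels the kart when airborne and animates the steering wheel, while Drift swaps per-side wheel classes at runtime.
; Damage triggers a timed slowdown and a timeline spinout using a stand-in mesh; the Clipper AOE is stubbed.
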(event `Spinout`
  (bind (_relativerotation_roll _relativerotation_pitch _relativerotation_yaw) (`KismetMathLibrary.BreakRotator` (`SceneComponent.RelativeRotation` (`self.spinmesh`))))
  (bind (_relativerotation_roll_2 _relativerotation_pitch_2) (`KismetMathLibrary.BreakRotator` (`SceneComponent.RelativeRotation` (`self.spinmesh`))))
  ;[1 1 1] Julia - spinout?
  (set `self.Spin` true)
  (set `self.KartOriginSpin` _relativerotation_yaw)
  (`SceneComponent.SetVisibility` (`self.Mesh`) false false)
  (`SceneComponent.SetVisibility` (`self.spinmesh`) true false)
  (bind (_direction _newtrack_0) (`Timeline|Timeline_0` :!via `PlayFromStart`)
    (:`Update`
      (bind _returnvalue (+ (* _newtrack_0 360.0) (`self.KartOriginSpin`)))
      (`SceneComponent.K2_SetRelativeRotation` (`self.spinmesh`) (`KismetMathLibrary.MakeRotator` _relativerotation_roll_2 _relativerotation_pitch_2 _returnvalue) false false)
      (`SceneComponent.K2_SetRelativeRotation` (`self.Char`) (`KismetMathLibrary.MakeRotator` _relativerotation_roll_2 _relativerotation_pitch_2 _returnvalue) false false))
    (:`Finished`
      (`SceneComponent.SetVisibility` (`self.Mesh`) true false)
      (`SceneComponent.SetVisibility` (`self.spinmesh`) false false)
      (set `self.Spin` false))))

(event `InputAction|HandBrake`
  (params (Key :type "Key Structure"))
  (bind _vehiclemovement (`self.VehicleMovement`))
  ;[0.8997 0.1041 1] Controls - Karl
  (:`Pressed`
    (`WheeledVehicleMovementComponent.SetHandbrakeInput` _vehiclemovement true))
  (:`Released`
    (`WheeledVehicleMovementComponent.SetHandbrakeInput` _vehiclemovement false)))

(event `CornerSlow`
  (params (ThrottleInput :type "Float (double-precision)") (BrakeInput :type "Float (double-precision)") (ThrottleOutput :type "Float (double-precision)") (BrakeDuration :type "Float (double-precision)"))
  (`self.SlowdownMacro` ThrottleInput BrakeInput ThrottleOutput BrakeDuration))

(event `self.ReceiveTick`
  (params (DeltaSeconds :type "Float (single-precision)"))
  (bind (_returnvalue_roll _returnvalue_pitch _returnvalue_yaw) (`KismetMathLibrary.BreakRotator` (`self.K2_GetActorRotation`)))
  (bind _returnvalue (`GameplayStatics.GetWorldDeltaSeconds`))
  (bind _returnvalue_2 (`self.GetInputAxisValue`))
  (bind _roll (.roll (`self.Steering Home`)))
  ;[0.8997 0.1041 1] Airtime - Karl
  (`self.AirTime`)
  (if (`self.InAir`)
    (`self.K2_SetActorRelativeRotation` (`KismetMathLibrary.MakeRotator` (`KismetMathLibrary.FInterpTo` _returnvalue_roll 0.0 _returnvalue (`self.Interp Speed`)) (`KismetMathLibrary.FInterpTo` _returnvalue_pitch 0.0 _returnvalue (`self.Interp Speed`)) _returnvalue_yaw) true true))
  (set `self.IsTurningLeft` (< _returnvalue_2 0.0))
  (set `self.IsTurningRight` (> _returnvalue_2 0.0))
  (set `self.IsNotTurning` (== _returnvalue_2 0.0))
  (set `self.Steering Amount` (`KismetMathLibrary.FInterpTo` (`self.Steering Amount`) (* _returnvalue_2 50.0) (`GameplayStatics.GetWorldDeltaSeconds`) 5.0))
  (`SceneComponent.K2_SetRelativeRotation` (`self.Steering Wheel`) (`KismetMathLibrary.MakeRotator` _roll (+ _roll (`self.Steering Amount`)) (.yaw (`self.Steering Home`))) false false))

(event `self.ReceiveBeginPlay`
  (set `self.Steering Home` (`SceneComponent.RelativeRotation` (`self.Steering Wheel`))))

(event `InputAction|Use Item`
  (params (Key :type "Key Structure"))
  ;[1 1 1] Item Usage - Julia
  (:`Pressed`
    (`|ExecutionSequence`
      (:`then_0`
        (switch `/Game/Items/Items` (`self.Item`)
          (:`NewEnumerator0`
            (`self.UseBanana`))
          (:`NewEnumerator1`
            (`self.UseRedShell`))
          (:`NewEnumerator3`
            (`self.UseGreenShell`))
          (:`NewEnumerator4`
            ;;[1 1 1] Clipper - Julia
            (if true
              (`self.Spawn AOE` (`self.K2_GetActorLocation`) 400.0 true self (delegate `CustomEvent_0`) 2.5 (struct :`G` 1.0 :`B` 0.091968 :`A` 1.0))))))
      (:`then_1`
        (set `self.Item` "NewEnumerator2")
        (set `self.ItemHeld` "")))))

(event `CustomEvent_0`
  (params (HitActor :type "Actor Object Reference"))
  ;[1 1 1] Item Usage - Julia
  ;;[1 1 1] Clipper - Julia
)

(fn `AddBoost`
  (params (BoostValue :type Integer))
  (bind _returnvalue (+ BoostValue (`self.CurrentBoost`)))
  ;[0.8997 0.1041 1] AddBoost - Karl
  (if (>= _returnvalue (`self.MaxBoost`))
    (set `self.CurrentBoost` (`self.MaxBoost`))
    (else
      (set `self.CurrentBoost` _returnvalue))))

(fn `AddHealth`
  (params (HealthValue :type Integer))
  (bind _returnvalue (+ HealthValue (`self.CurrentHealth`)))
  ;[0.8997 0.1041 1] AddHealth - Karl
  (if (>= _returnvalue (`self.MaxHealth`))
    (set `self.CurrentHealth` (`self.MaxHealth`))
    (else
      (set `self.CurrentHealth` _returnvalue))))

(fn `AirTime`
  (locals (SetIsInAir :type Boolean :default true))
  ;[0.8997 0.1041 1] Air Time - Karl
  (for _array_element (`WheeledVehicleMovementComponent.Wheels` (`self.VehicleMovement`))
    (if (`VehicleWheel.IsInAir` _array_element)
      (if (`local.SetIsInAir`) :!label _label
        (set `self.InAir` true)
        (else
          (set `self.InAir` false)))
      (else
        (set `local.SetIsInAir` false))))
  (goto _label))

(fn `AntiFlipV1(Unused)`
  (bind (_returnvalue_roll _returnvalue_pitch _returnvalue_yaw) (`KismetMathLibrary.BreakRotator` (`self.K2_GetActorRotation`)))
  ;[0.8997 0.1041 1] Antip Flip V1 - Karl
  (if (> _returnvalue_roll 20.0)
    (`self.K2_SetActorRelativeRotation` (`KismetMathLibrary.MakeRotator` (`KismetMathLibrary.FInterpTo` _returnvalue_roll 0.0 (`GameplayStatics.GetWorldDeltaSeconds`) 100.0) _returnvalue_pitch _returnvalue_yaw))))

(fn `AntiFlipV2(Unused)`
  (bind _roll (.roll (`self.K2_GetActorRotation`)))
  ;[0.8997 0.1041 1] AntipFlipV2 - Karl
  (if (> _roll 10.0)
    (set `self.RollRotation` 20.0)
    (`self.K2_SetActorRotation` (`KismetMathLibrary.MakeRotator` (`self.RollRotation`) (.pitch (`self.K2_GetActorRotation`)) (.yaw (`self.K2_GetActorRotation`))) true :!label _label)
    (`KismetSystemLibrary.PrintString` (`KismetStringLibrary.Conv_RotatorToString` (`self.K2_GetActorRotation`)))
    (elif (< _roll -10.0)
      (set `self.RollRotation` -20.0)
      (else
        (set `self.RollRotation` _roll)
        (goto _label)))))

(fn `Boost`
  (bind _returnvalue (* (`self.GetActorForwardVector`) 150.0))
  ;[0.8997 0.1041 1] Boost - Katl
  (if (< (`KismetMathLibrary.VSize` _returnvalue) (`self.MaxVelocity`))
    (`PrimitiveComponent.SetPhysicsLinearVelocity` (`MovementComponent.UpdatedPrimitive` (`self.VehicleMovement`)) _returnvalue true "None")))

(fn `Brake`
  (params (BrakeInput :type "Float (double-precision)"))
  (`WheeledVehicleMovementComponent.SetBrakeInput` (`self.VehicleMovement`) BrakeInput))

(fn `Char Position`
  (params (`New Rotation X (Roll)` :type "Float (double-precision)") (`New Rotation Y (Pitch)` :type "Float (double-precision)") (`New Rotation Z (Yaw)` :type "Float (double-precision)") (`New Location X` :type "Float (double-precision)") (`New Location Y` :type "Float (double-precision)") (`New Location Z` :type "Float (double-precision)"))
  (returns (Char :type "SkeletalMeshComponent Object Reference"))
  (bind _char (`self.Char`))
  (`SceneComponent.K2_SetRelativeRotation` _char (`KismetMathLibrary.MakeRotator` `New Rotation X (Roll)` `New Rotation Y (Pitch)` `New Rotation Z (Yaw)`) false false)
  (`SceneComponent.K2_SetRelativeLocation` _char (`KismetMathLibrary.MakeVector` `New Location X` `New Location Y` `New Location Z`) false false)
  (return _char))

(fn `Char Swap`
  (params (Character :type "SkeletalMesh Object Reference") (AnimBP :type "Object Class Reference"))
  (`SkinnedMeshComponent.SetSkinnedAssetAndUpdate` (`self.Char`) Character true)
  (`SkeletalMeshComponent.SetAnimInstanceClass` (`self.Char`) AnimBP)
  (`SkeletalMeshComponent.SetAnimationMode` (`self.Char`) "AnimationBlueprint"))

(fn `DealDamage`
  (params (Damage :type Integer))
  (returns (RespawnKart :type Boolean))
  ;[0.8997 0.1041 1] Deal Damage - Karl
  (bind _output_get (set `self.CurrentHealth` (- (`self.CurrentHealth`) Damage)))
  (`self.Spinout`)
  (`self.Slowdown` 0.2 1.0 1.0 2.0)
  (return (<= _output_get 0)))

(fn `Drift`
  (params (IsDrifting :type Boolean) (Velocity :type "Vector Structure") (Gear :type Integer))
  (locals (FL :type Boolean) (FR :type Boolean) (RL :type Boolean) (RR :type Boolean))
  (bind _returnvalue (`self.GetInputAxisValue`))
  (if IsDrifting
    ;[1 1 1] If Steer Right
    (if (> _returnvalue 0.0)
      (set `local.FL` true)
      (set `local.FR` false)
      (set `local.RL` true)
      (set `local.RR` false)
      (`KismetSystemLibrary.PrintString` "Right")
      (`TireLib.modifyTyreConfig` (`self.VehicleMovement`) (`|MakeArray` (make `WheelSetupBp` (select `bool` (`local.FL`) :`false` (`self.frontWheels`) :`true` (`self.DriftFrontWheels`)) "FL") (make `WheelSetupBp` (select `bool` (`local.FR`) :`false` (`self.frontWheels`) :`true` (`self.DriftFrontWheels`)) "FR") (make `WheelSetupBp` (select `bool` (`local.RL`) :`false` (`self.frontWheels`) :`true` (`self.DriftFrontWheels`)) "RL" (0.0 0.0 0.0) true) (make `WheelSetupBp` (select `bool` (`local.RR`) :`false` (`self.frontWheels`) :`true` (`self.DriftFrontWheels`)) "RR" (0.0 0.0 0.0) true)) :!label _label)
      (`PrimitiveComponent.SetAllPhysicsLinearVelocity` (`self.Mesh`) Velocity false)
      (`WheeledVehicleMovementComponent.SetTargetGear` (`self.VehicleMovement`) Gear true)
      (else
        ;[1 1 1] If Steer Left
        (if (< _returnvalue 0.0)
          (set `local.FL` false)
          (set `local.FR` true)
          (set `local.RL` false)
          (set `local.RR` true)
          (`KismetSystemLibrary.PrintString` "Left")
          (goto _label)
          (elif (== _returnvalue 0.0)
            (set `local.FL` false)
            (set `local.FR` false)
            (set `local.RL` false)
            (set `local.RR` false)
            (`KismetSystemLibrary.PrintString` "Straight")
            (goto _label)))))
    (else
      (set `local.FL` false)
      (set `local.FR` false)
      (set `local.RL` false)
      (set `local.RR` false)
      (goto _label))))

(fn `Handbrake`
  (params (HandbrakeIn :type Boolean))
  ;[0.8997 0.1041 1] Handbrake - Karl
  (if HandbrakeIn
    (`WheeledVehicleMovementComponent.SetHandbrakeInput` (`self.VehicleMovement`) true)
    (else
      (`WheeledVehicleMovementComponent.SetHandbrakeInput` (`self.VehicleMovement`) false)))
  (return))

(fn `KartSwap`
  (params (Kart :type Name))
  (bind _returnvalue (`|GetDataTableRow` "/Game/Kart/KartV4/Blueprints/KartData.KartData" Kart)
    (:`then`
      (`SkinnedMeshComponent.SetSkinnedAssetAndUpdate` (`self.Mesh`) (break `/Game/Kart/KartV4/Blueprints/KartStruct` _returnvalue) true)
      (`SkeletalMeshComponent.SetAnimInstanceClass` (`self.Mesh`) (`.AnimationBP_7_ADE3A0FE443F6733A9083A869A835508` (break `/Game/Kart/KartV4/Blueprints/KartStruct` _returnvalue)))
      (`SkeletalMeshComponent.SetAnimationMode` (`self.Mesh`) "AnimationBlueprint")
      (set `self.DriftFrontWheels` (`.DriftFrontWheels_13_CD4B58FE4C379CCEF7AA35A3844F8F8F` (break `/Game/Kart/KartV4/Blueprints/KartStruct` _returnvalue)))
      (bind _output_get (set `self.frontWheels` (`.FrontWheels_12_2937D88A4C31607A3D9BD98667999F78` (break `/Game/Kart/KartV4/Blueprints/KartStruct` _returnvalue))))
      (bind _output_get_2 (set `self.RearWheels` (`.RearWheels_17_2C6558194806D994FD3E5D8CC2600CE3` (break `/Game/Kart/KartV4/Blueprints/KartStruct` _returnvalue))))
      (set `self.DriftRearWheels` (`.DriftRearWheels_15_408ACA3044958F4FEA73AA83D0D0136C` (break `/Game/Kart/KartV4/Blueprints/KartStruct` _returnvalue)))
      (`StaticMeshComponent.SetStaticMesh` (`self.spinmesh`) (`.SpinOutMesh_20_226FF1C44DAC81715FF2059D69CA27E0` (break `/Game/Kart/KartV4/Blueprints/KartStruct` _returnvalue)))
      (`self.ModifyWheels` _output_get _output_get _output_get_2 _output_get_2))))

(fn `ModifyWheels`
  (params (`Front Left` :type "VehicleWheel Class Reference") (`Front Right` :type "VehicleWheel Class Reference") (`Rear Left` :type "VehicleWheel Class Reference") (`Rear Right` :type "VehicleWheel Class Reference"))
  (`TireLib.modifyTyreConfig` (`self.VehicleMovement`) (`|MakeArray` (make `WheelSetupBp` `Front Left` "FL") (make `WheelSetupBp` `Front Right` "FR") (make `WheelSetupBp` `Rear Left` "RL" (0.0 0.0 0.0) true) (make `WheelSetupBp` `Rear Right` "RR" (0.0 0.0 0.0) true))))

(fn `Slowdown`
  (params (ThrottleInput :type "Float (double-precision)") (ThrottleOutput :type "Float (double-precision)") (BrakeForce :type "Float (double-precision)") (BrakeLength :type "Float (double-precision)"))
  ;[0.8997 0.1041 1] Slowdown - Karl
  (`self.CornerSlow` ThrottleInput BrakeForce ThrottleOutput BrakeLength)
  (return))

(fn `Spawn AOE`
  (params (Location :type "Vector Structure") (Radious :type "Float (double-precision)") (`Line of sight ` :type Boolean) (`AOE start ` :type "Actor Object Reference") (HitEvent :type "Delegate (by ref)") (`Debug duration` :type "Float (double-precision)") (`Debug colour` :type "LinearColor Structure")))

(fn `Steering`
  (params (SteeringInput :type "Float (double-precision)"))
  (returns (SteeringOutput :type "Float (double-precision)"))
  ;[0.8997 0.1041 1] Steering - Karl
  (`WheeledVehicleMovementComponent.SetSteeringInput` (`self.VehicleMovement`) SteeringInput)
  (return SteeringInput))

(fn `Throttle`
  (params (ThrottleInput :type "Float (double-precision)"))
  (returns (ThrottleOutput :type "Float (double-precision)"))
  ;[0.8997 0.1041 1] Throttle - Karl
  (`WheeledVehicleMovementComponent.SetThrottleInput` (`self.VehicleMovement`) ThrottleInput)
  (return ThrottleInput))

(fn `UseBanana`
  ;[1 1 1] Banana - Julia
  (if (`self.Has Bananana`)
    (`|SpawnActorFromClass` "/Game/Items/Banana/Bananana.Bananana_C" (`SceneComponent.K2_GetComponentToWorld` (`self.Banana spawn`)) "Undefined" "OverrideRootScale" null null)
    (set `self.Has Bananana` false)))

(fn `UseClipper`)

(fn `UseGreenShell`
  ;[1 1 1] Green Shell - Julia
  (if (`self.Has GreenShell`)
    (`|SpawnActorFromClass` "/Game/Items/Green_Shell.Green_Shell_C" (`KismetMathLibrary.MakeTransform` (.location (`SceneComponent.K2_GetComponentToWorld` (`self.Shell spawn`))) (.rotation (`SceneComponent.K2_GetComponentToWorld` (`self.Shell spawn`))) (15.0 15.0 15.0)) "Undefined" "OverrideRootScale" null null)
    (set `self.Has GreenShell` false)))

(fn `UserConstructionScript`
  (bind _mesh (`self.Mesh`))
  (bind _spinmesh (`self.spinmesh`))
  (bind _mesh_2 (`self.Mesh`))
  (bind _spinmesh_2 (`self.spinmesh`))
  (bind _steering_wheel (`self.Steering Wheel`))
  (bind (_relativerotation_roll _relativerotation_pitch) (`KismetMathLibrary.BreakRotator` (`SceneComponent.RelativeRotation` _steering_wheel)))
  (if (`self.IsPlayer`)
    (bind _asjmgame_instance (cast `/Game/JMGameInstance` (`GameplayStatics.GetGameInstance`)))
    (set `self.KartSelector` (`/Game/JMGameInstance.KartSelector` _asjmgame_instance)))
  (switch `name` (`self.KartSelector`)
    (:`Default`
      (`self.KartSwap` "Matra" :!label _label)
      (`SceneComponent.K2_AttachToComponent` (`self.Steering Wheel`) (`self.Mesh`) "SteeringWheel" "SnapToTarget" "SnapToTarget" "SnapToTarget" true :!label _label_2))
    (:`Matra`
      (goto _label))
    (:`Rx7`
      (`self.KartSwap` "RX7")
      (goto _label_2))
    (:`PeachKart`
      (`self.KartSwap` "PeachKart")
      (goto _label_2))
    (:`LuigiKart`
      (`self.KartSwap` "LuigiKart")
      (goto _label_2))
    (:`KoopaKart`
      (`self.KartSwap` "KoopaKart")
      (goto _label_2))
    (:`BowserKart`
      (`self.KartSwap` "BowserKart")
      (`SceneComponent.K2_AttachToComponent` (`self.Steering Wheel`) (`self.Mesh`) "SteeringWheel2" "SnapToTarget" "SnapToTarget" "SnapToTarget" true))
    (:`Rose`
      ;[1 1 1] Rose
      (`self.KartSwap` "PeachKart")
      (`PrimitiveComponent.SetMaterial` _mesh 0 "/Game/CharactersAndKarts/Karts/RoselinaKart/Textures/Interior/M_Interior.M_Interior")
      (`PrimitiveComponent.SetMaterial` _mesh 1 "/Game/CharactersAndKarts/Karts/RoselinaKart/Textures/Body/M_RoselinaKartBody.M_RoselinaKartBody")
      (`PrimitiveComponent.SetMaterial` _mesh 2 "/Game/CharactersAndKarts/Karts/RoselinaKart/Textures/Trim/Trim.Trim")
      (`PrimitiveComponent.SetMaterial` _spinmesh 0 "/Game/CharactersAndKarts/Karts/RoselinaKart/Textures/Interior/M_Interior.M_Interior")
      (`PrimitiveComponent.SetMaterial` _spinmesh 1 "/Game/CharactersAndKarts/Karts/RoselinaKart/Textures/Body/M_RoselinaKartBody.M_RoselinaKartBody")
      (`PrimitiveComponent.SetMaterial` _spinmesh 2 "/Game/CharactersAndKarts/Karts/RoselinaKart/Textures/Trim/Trim.Trim")
      (goto _label_2))
    (:`Daisy`
      ;[1 1 1] Daisy
      (`self.KartSwap` "PeachKart")
      (`PrimitiveComponent.SetMaterial` _mesh_2 0 "/Game/CharactersAndKarts/Karts/DaisyKart/Interior/M_DaisyKartInterior.M_DaisyKartInterior")
      (`PrimitiveComponent.SetMaterial` _mesh_2 1 "/Game/CharactersAndKarts/Karts/DaisyKart/Body/M_DaisyKartBody.M_DaisyKartBody")
      (`PrimitiveComponent.SetMaterial` _mesh_2 2 "/Game/CharactersAndKarts/Karts/DaisyKart/Trim/M_DaisyKartTrim.M_DaisyKartTrim")
      (`PrimitiveComponent.SetMaterial` _spinmesh_2 0 "/Game/CharactersAndKarts/Karts/DaisyKart/Interior/M_DaisyKartInterior.M_DaisyKartInterior")
      (`PrimitiveComponent.SetMaterial` _spinmesh_2 1 "/Game/CharactersAndKarts/Karts/DaisyKart/Body/M_DaisyKartBody.M_DaisyKartBody")
      (`PrimitiveComponent.SetMaterial` _spinmesh_2 2 "/Game/CharactersAndKarts/Karts/DaisyKart/Trim/M_DaisyKartTrim.M_DaisyKartTrim")
      (goto _label_2)))
  (`SceneComponent.K2_SetRelativeRotation` _steering_wheel (`KismetMathLibrary.MakeRotator` _relativerotation_roll _relativerotation_pitch -90.0) false false)
  (if (`self.IsPlayer`)
    (bind _asjmgame_instance_2 (cast `/Game/JMGameInstance` (`GameplayStatics.GetGameInstance`)))
    (set `self.CharSelector` (`/Game/JMGameInstance.CharacterSelector` _asjmgame_instance_2)))
  (switch `int` (`self.CharSelector`)
    (:`Default`
      (`self.Char Swap` "/Game/CompletedRigs_CharactersAndKarts/CharacterRigs/Luigi_Rig/Luigi_Rig/luigi_rig.luigi_rig" "/Game/CompletedRigs_CharactersAndKarts/CharacterRigs/Luigi_Rig/Luigi_Rig/Luigi_rig_AnimBP.Luigi_rig_AnimBP_C" :!label _label_3))
    (:`0`
      (goto _label_3))
    (:`1`
      (`self.Char Swap` "/Game/CompletedRigs_CharactersAndKarts/CharacterRigs/Peach_Rig/Peach_Rig.Peach_Rig" "/Game/CompletedRigs_CharactersAndKarts/KarlBigBodgeAnims/Peach/PeachAnimBP.PeachAnimBP_C"))
    (:`2`
      (`self.Char Swap` "/Game/CompletedRigs_CharactersAndKarts/CharacterRigs/Waluigi_Rig/Waluigi_Rig.Waluigi_Rig" "/Game/CompletedRigs_CharactersAndKarts/KarlBigBodgeAnims/wal/WaluigiAnimBP.WaluigiAnimBP_C")
      (set `self.IsWal` true))
    (:`3`
      (`self.Char Swap` "/Game/CompletedRigs_CharactersAndKarts/CharacterRigs/Mario_Rig/Mario_Rig_V1.Mario_Rig_V1" "/Game/CompletedRigs_CharactersAndKarts/KarlBigBodgeAnims/mario/Mario_rig_AnimBP.Mario_rig_AnimBP_C"))
    (:`4`
      (`self.Char Swap` "/Game/CompletedRigs_CharactersAndKarts/CharacterRigs/Peach_Rig/Peach_Rig.Peach_Rig" "/Game/CompletedRigs_CharactersAndKarts/KarlBigBodgeAnims/Peach/PeachAnimBP.PeachAnimBP_C")
      (`PrimitiveComponent.SetMaterial` (`self.Char`) 0 "/Game/CharactersAndKarts/Characters/Daisy/Textures/M_Daisy.M_Daisy"))
    (:`5`
      (`self.Char Swap` "/Game/CompletedRigs_CharactersAndKarts/CharacterRigs/Peach_Rig/Peach_Rig.Peach_Rig" "/Game/CompletedRigs_CharactersAndKarts/KarlBigBodgeAnims/Peach/PeachAnimBP.PeachAnimBP_C")
      (`PrimitiveComponent.SetMaterial` (`self.Char`) 0 "/Game/CharactersAndKarts/Characters/Roselina/Textures/M_Roselina.M_Roselina"))
    (:`6`
      (`self.Char Swap` "/Game/CompletedRigs_CharactersAndKarts/CharacterRigs/Bowser_Rig/Bowser_Rig_V0_9.Bowser_Rig_V0_9" "/Game/CompletedRigs_CharactersAndKarts/KarlBigBodgeAnims/Bowser/Bowser_Probs_wont_work_rig_AnimBP.Bowser_Probs_wont_work_rig_AnimBP_C")))
  (`SceneComponent.K2_AttachToComponent` (`self.Char`) (`self.Mesh`) "Seat1" "SnapToTarget" "SnapToTarget" "SnapToTarget" true)
  (if (`self.IsWal`)
    (switch `name` (`self.KartSelector`)
      (:`Matra`
        (`self.Char Position` 0.0 0.0 -90.0 20.0 0.0 -15.0))
      (:`Rx7`
        (`self.Char Position` 0.0 0.0 -90.0 20.0))
      (:`PeachKart`
        (`self.Char Position` 0.0 0.0 -90.0 30.0 0.0 -20.0 :!label _label_4))
      (:`LuigiKart`
        (`self.Char Position` 0.0 0.0 -90.0 30.0 0.0 -50.0))
      (:`KoopaKart`
        (`self.Char Position` 0.0 0.0 -90.0))
      (:`BowserKart`
        (`self.Char Position` 0.0 0.0 -90.0 30.0 0.0 -29.0))
      (:`Rose`
        (goto _label_4))
      (:`Daisy`
        (goto _label_4)))
    (else
      (switch `name` (`self.KartSelector`)
        (:`Matra`
          (`self.Char Position` 0.0 0.0 -90.0 -15.0 0.0 -15.0))
        (:`Rx7`
          (`self.Char Position` 0.0 0.0 -90.0 -15.0))
        (:`PeachKart`
          (`self.Char Position` 0.0 0.0 -90.0 0.0 0.0 -20.0 :!label _label_5))
        (:`LuigiKart`
          (`self.Char Position` 0.0 0.0 -90.0 10.0 0.0 -50.0))
        (:`KoopaKart`
          (`self.Char Position` 0.0 0.0 -90.0 -40.0))
        (:`BowserKart`
          (`self.Char Position` 0.0 0.0 -90.0 -10.0 0.0 -20.0))
        (:`Rose`
          (goto _label_5))
        (:`Daisy`
          (goto _label_5))))))

(fn `UseRedShell`
  ;[1 1 1] Shell - Julia
  (if (`self.Has Shell`)
    (`|SpawnActorFromClass` "/Game/Items/Red_Shell.Red_Shell_C" (`KismetMathLibrary.MakeTransform` (.location (`SceneComponent.K2_GetComponentToWorld` (`self.Shell spawn`))) (.rotation (`SceneComponent.K2_GetComponentToWorld` (`self.Shell spawn`))) (15.0 15.0 15.0)) "Undefined" "OverrideRootScale" null null)
    (set `self.Has Shell` false)))